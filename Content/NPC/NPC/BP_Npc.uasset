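; BP_Npc is an NPC that deals repeated damage to the third-person player character while it stays in range.
; BeginPlay records two patrol points from the spawn location and an offset, and negates the damage amount.
; Overlapping DamageRange stores the player and loops UpdateHealth with a cooldown Delay until end overlap clears that reference.
; No movement logic in these graphs uses the patrol points.
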(event OnComponentBeginOverlap(DamageRange)
  (params (OverlappedComponent :type Primitive%20Component%20Object%20Reference) (OtherActor :type Actor%20Object%20Reference) (OtherComp :type Primitive%20Component%20Object%20Reference) (OtherBodyIndex :type Integer) (bFromSweep :type Boolean) (SweepResult :type Hit%20Result%20Structure%20%28by%20ref%29))
  (bind _asbp_third_person_character (Utilities|Casting|CastToBP_ThirdPersonCharacter OtherActor))
  (bind _output_get (Variables|Default|SetTargetPlayerCharacter _asbp_third_person_character))
  (Default|UpdateHealth _output_get (Variables|Default|GetDamageAmount) :!label _label)
  (Utilities|FlowControl|Delay (Variables|Default|GetCooldown))
  (Utilities|IsValid (Variables|Default|GetTargetPlayerCharacter)
    (:Is%20Valid
      (goto _label))))

(event OnComponentEndOverlap(DamageRange)
  (params (OverlappedComponent :type Primitive%20Component%20Object%20Reference) (OtherActor :type Actor%20Object%20Reference) (OtherComp :type Primitive%20Component%20Object%20Reference) (OtherBodyIndex :type Integer))
  (Utilities|Casting|CastToBP_ThirdPersonCharacter OtherActor)
  (Variables|Default|SetTargetPlayerCharacter 0))

(event EventBeginPlay
  (bind _returnvalue (Transformation|GetActorLocation))
  (Variables|Default|Setpotrolpoint1 _returnvalue)
  (Variables|Default|Setpotrolpoint2 (+ _returnvalue (Variables|Default|Getpotrolpoint2)))
  (Variables|Default|SetDamageAmount (* (Variables|Default|GetDamageAmount) -1.0)))

(fn ConstructionScript)